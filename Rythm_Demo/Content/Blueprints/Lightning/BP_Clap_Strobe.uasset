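; Strobe light Blueprint that runs a timed, three-phase flashing sequence on its light component, starting at BeginPlay.
; It hides the light until a configurable StartDelay elapses, then reveals it and starts the first strobe timeline.
; Three timelines drive light intensity in turn, chained by hardcoded delays with pauses between phases.
; The first two are explicitly stopped, while the third has no stop call.
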(event EventBeginPlay
  (bind _lightcomponent (Variables|Default|GetLightComponent))
  (Development|SetHiddeninGame _lightcomponent true true)
  (Utilities|FlowControl|Delay (Variables|Config|GetStartDelay))
  (Development|SetHiddeninGame _lightcomponent false true)
  (Utilities|FlowControl|Sequence
    (:then_0
      (bind _intensity (Timeline|Strobe_01 SetNewTime)
        (:Update
          (Rendering|Components|Light|SetIntensity _lightcomponent _intensity))))
    (:then_1
      (Timeline|Strobe_01 Play))
    (:then_2
      (Utilities|FlowControl|Delay 11.8)
      (Utilities|FlowControl|Sequence
        (:then_0
          (Timeline|Strobe_01 Stop))
        (:then_1
          (Utilities|FlowControl|Delay 13.8)
          (Utilities|FlowControl|Sequence
            (:then_0
              (bind _intensity_2 (Timeline|Strobe_02 SetNewTime)
                (:Update
                  (Rendering|Components|Light|SetIntensity _lightcomponent _intensity_2))))
            (:then_1
              (Timeline|Strobe_02 Play))
            (:then_2
              (Utilities|FlowControl|Delay 5.6)
              (Utilities|FlowControl|Sequence
                (:then_0
                  (Timeline|Strobe_02 Stop))
                (:then_1
                  (Utilities|FlowControl|Delay 0.8)
                  (Utilities|FlowControl|Sequence
                    (:then_0
                      (bind _intensity_3 (Timeline|Strobe_03 SetNewTime)
                        (:Update
                          (Rendering|Components|Light|SetIntensity _lightcomponent _intensity_3))))
                    (:then_1
                      (Timeline|Strobe_03 Play))))))))))))

(fn ConstructionScript)